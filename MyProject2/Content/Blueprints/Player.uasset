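; Player Blueprint for a flyer that moves constantly forward while the player strafes sideways and vertically.
; AxisX and AxisY feed movement input along the actor's right and up vectors.
; Tick consumes that input, scales it by StrafeSpeed, adds forward motion at FlightSpeed, and offsets PlayerRoot frame-rate independently without sweep.
; A SpawnTunnel function spawns an actor at a given location but is not called within this Blueprint.
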(event EventBeginPlay)

(event Collision|EventActorBeginOverlap
  (params (OtherActor :type Actor%20Object%20Reference)))

(event EventTick
  (params (DeltaSeconds :type Float%20%28single-precision%29))
  (bind _returnvalue (Class|Pawn|ConsumeMovementInputVector))
  (Transformation|AddLocalOffset (Variables|Default|GetPlayerRoot) (+ (* _returnvalue (* DeltaSeconds (Variables|Default|GetStrafeSpeed))) (* (Transformation|GetActorForwardVector) (* DeltaSeconds (Variables|Default|GetFlightSpeed)))) false false))

(event Input|AxisEvents|InputAxisAxisX
  (params (AxisValue :type Float%20%28single-precision%29))
  (Pawn|Input|AddMovementInput (Transformation|GetActorRightVector) AxisValue false))

(event Input|AxisEvents|InputAxisAxisY
  (params (AxisValue :type Float%20%28single-precision%29))
  (Pawn|Input|AddMovementInput (Transformation|GetActorUpVector) AxisValue false))

(fn ConstructionScript)

(fn SpawnTunnel
  (params (Location :type Vector))
  (Game|SpawnActorfromClass "/Game/Blueprints/Tunnel.Tunnel_C" (Math|Transform|MakeTransform Location "0, 0, 0" "1,1,1") "Undefined" 0 0))